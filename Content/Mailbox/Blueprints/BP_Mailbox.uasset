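; Mailbox actor that opens a mail UI for the player who interacts with it and announces new mail.
; Opening creates a WBP_Mailbox widget for the interactor's player controller and disables the Interactable until the widget's OnClosed re-enables it.
; A change to unread mail prints a notice, and EndPlay closes any open widget.
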(event `self.OnUnreadChanged`
  (params (bHasUnread :type Boolean))
  (if bHasUnread
    (`KismetSystemLibrary.PrintString` "You've got mail!")))

(event `self.OnOpened`
  (params (Interactor :type "Actor Object Reference"))
  (bind _ascharacter (cast `Character` Interactor))
  (bind _asplayer_controller (cast `PlayerController` (`Pawn.GetController` _ascharacter)))
  (bind _returnvalue (`|CreateWidget` "/Game/Mailbox/Widgets/WBP_Mailbox.WBP_Mailbox_C" _asplayer_controller))
  (add `/Game/Mailbox/Widgets/WBP_Mailbox.OnClosed` _returnvalue (delegate `OnClosed`))
  (bind _output_get (set `self.WBP_Mailbox` _returnvalue))
  (`UserWidget.AddToViewport` _returnvalue 0)
  (`UserWidget.AddToViewport` _output_get 0)
  (set `NenInteractableComponent.bEnabled` false (`self.Interactable`)))

(event `self.ReceiveEndPlay`
  (params (EndPlayReason :type "EEndPlayReason Enum" :default "Destroyed"))
  (bind _wbp_mailbox (`self.WBP_Mailbox`))
  (if (`KismetSystemLibrary.IsValid` _wbp_mailbox)
    (`/Game/Mailbox/Widgets/WBP_Mailbox.Close` _wbp_mailbox)))

(event `OnClosed`
  (set `NenInteractableComponent.bEnabled` true (`self.Interactable`))
  (set `self.WBP_Mailbox` null))

(fn `UserConstructionScript`)